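; BP_Car is a car actor that travels along the first BP_Spline found in the level, starting at BeginPlay.
; The Move timeline, rate-scaled by TimeToComplete, maps its track to spline distance and updates the actor transform.
; Location is sampled in world space, but rotation in local space.
; Any Box overlap destroys the car, then enables mesh physics on the already destroyed actor.
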(event `self.ReceiveBeginPlay`
  (bind _returnvalue (`GameplayStatics.GetActorOfClass` "/Game/BP_Spline.BP_Spline_C"))
  (set `self.Spline Ref` _returnvalue)
  (`self.Move Car`))

(event `Move Car`
  (bind _spline (`/Game/BP_Spline.Spline` (`self.Spline Ref`)))
  (`TimelineComponent.SetPlayRate` (`self.Move`) (/ 1.0 (`self.Time To Complete`)))
  (bind (_direction _move_track) (`Timeline|Move`)
    (:`Update`
      (bind _returnvalue (`KismetMathLibrary.Lerp` 0.0 (`SplineComponent.GetSplineLength` (`/Game/BP_Spline.Spline` (`self.Spline Ref`))) _move_track))
      (`self.K2_SetActorTransform` (`KismetMathLibrary.MakeTransform` (`SplineComponent.GetLocationAtDistanceAlongSpline` _spline _returnvalue "World") (`SplineComponent.GetRotationAtDistanceAlongSpline` _spline _returnvalue "Local"))))))

(event `self.Box.OnComponentBeginOverlap`
  (params (OverlappedComponent :type "PrimitiveComponent Object Reference") (OtherActor :type "Actor Object Reference") (OtherComp :type "PrimitiveComponent Object Reference") (OtherBodyIndex :type Integer) (bFromSweep :type Boolean) (SweepResult :type "HitResult Structure (by ref)"))
  (`self.K2_DestroyActor`)
  (`PrimitiveComponent.SetSimulatePhysics` (`self.StaticMesh`) true))

(fn `UserConstructionScript`)