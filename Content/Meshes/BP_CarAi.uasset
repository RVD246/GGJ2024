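; BP_CarAi is a car actor that loops along a spline and can be wrecked by a BP_Fraud character.
; A Timeline, rate-scaled by TimeToComplete, drives its transform; a repeating timer changes that duration when the spline is full, effective next lap.
; Overlapping launches a non-ragdolled BP_Fraud.
; High ragdoll velocity makes the car's Geometry Collection burst with effects, decrements the spline's count, boosts the character and destroys the car after a delay.
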(event `self.ReceiveBeginPlay`
  (`|ExecutionSequence`
    (:`then_0`
      (`KismetSystemLibrary.K2_SetTimer` null "SpeedCheck" 1.0 true))
    (:`then_1`
      (`self.Move car`))))

(event `Move car`
  (bind _spline (`/Game/BP_Spline.Spline` (`self.spline`)))
  (`TimelineComponent.SetPlayRate` (`self.move`) (/ 1.0 (`self.Time to complete`)))
  (bind (_direction _newtrack_0) (`Timeline|move` :!via `PlayFromStart`)
    (:`Update`
      (bind _returnvalue (`KismetMathLibrary.Lerp` 0.0 (`SplineComponent.GetSplineLength` (`/Game/BP_Spline.Spline` (`self.spline`))) _newtrack_0))
      (`self.K2_SetActorTransform` (`KismetMathLibrary.MakeTransform` (`SplineComponent.GetLocationAtDistanceAlongSpline` _spline _returnvalue "World") (`SplineComponent.GetRotationAtDistanceAlongSpline` _spline _returnvalue "Local"))))
    (:`Finished`
      (`self.Move car`))))

(event `self.Checker.OnComponentBeginOverlap`
  (params (OverlappedComponent :type "PrimitiveComponent Object Reference") (OtherActor :type "Actor Object Reference") (OtherComp :type "PrimitiveComponent Object Reference") (OtherBodyIndex :type Integer) (bFromSweep :type Boolean) (SweepResult :type "HitResult Structure (by ref)"))
  (bind _returnvalue (`self.K2_GetActorLocation`))
  (bind _geometrycollectioncomponent (`self.GeometryCollectionComponent`))
  (bind _asbp_fraud (cast `/Game/ThirdPerson/Blueprints/BP_Fraud` OtherActor))
  (if (not (`/Game/ThirdPerson/Blueprints/BP_Fraud.GetIsRagdoll` _asbp_fraud))
    (`/Game/ThirdPerson/Blueprints/BP_Fraud.LAUNCHER` _asbp_fraud))
  (if (> (`KismetMathLibrary.VSize` (`/Game/ThirdPerson/Blueprints/BP_Fraud.GetRagdollVelocity` _asbp_fraud)) 1200.0)
    (`PrimitiveComponent.SetSimulatePhysics` _geometrycollectioncomponent true)
    (`PrimitiveComponent.AddImpulse` _geometrycollectioncomponent (0.0 0.0 100000.0) "None" false)
    (`NiagaraFunctionLibrary.SpawnSystemAtLocation` "/Game/FX/P_Fart.P_Fart" _returnvalue)
    (`GameplayStatics.PlaySoundAtLocation` "/Game/StarterContent/Audio/Explosion_Cue.Explosion_Cue" _returnvalue (struct) 1.0 1.0 0.0 null null null null)
    (`ActorComponent.K2_DestroyComponent` (`self.Hitter`))
    (`ActorComponent.K2_DestroyComponent` (`self.Checker`))
    (`/Engine/EditorBlueprintResources/StandardMacros.DecrementInt` (`/Game/BP_Spline.Number of actors on spline` (`self.spline`))
      (:`  `
        (`PrimitiveComponent.AddImpulse` (`Character.Mesh` _asbp_fraud) (0.0 0.0 60000.0) "pelvis" false)
        (`KismetSystemLibrary.Delay` 5.0)
        (`self.K2_DestroyActor`)))))

(event `SpeedCheck`
  (bind _spline (`self.spline`))
  (if (== (`/Game/BP_Spline.Number of actors on spline` _spline) (`/Game/BP_Spline.Max actors on spline` _spline))
    (bind _output_get (set `self.Time to complete` 30.0))
    (`KismetSystemLibrary.PrintString` (`KismetStringLibrary.Conv_DoubleToString` _output_get))))

(fn `UserConstructionScript`)