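; Destructible Geometry Collection car that blows up on overlap, with logic to drive it along a spline.
; Movecar runs a timeline scaled by TimeToComplete to set location and rotation along SplineRef's spline.
; Box overlap enables physics, launches the car upward with effects and sound, spawns a replacement, then destroys it after a delay.
; The BP_Spline lookup and MoveCar call are disconnected, and BeginPlay is empty.
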(event `self.ReceiveBeginPlay`)

(event `Move car`
  (bind _spline (`/Game/BP_Spline.Spline` (`self.Spline Ref`)))
  (`TimelineComponent.SetPlayRate` (`self.move`) (/ 1.0 (`self.Time to complete`)))
  (bind (_direction _newtrack_0) (`Timeline|move`)
    (:`Update`
      (bind _returnvalue (`KismetMathLibrary.Lerp` 0.0 (`SplineComponent.GetSplineLength` (`/Game/BP_Spline.Spline` (`self.Spline Ref`))) _newtrack_0))
      (`self.K2_SetActorTransform` (`KismetMathLibrary.MakeTransform` (`SplineComponent.GetLocationAtDistanceAlongSpline` _spline _returnvalue "World") (`SplineComponent.GetRotationAtDistanceAlongSpline` _spline _returnvalue "Local"))))))

(event `self.Box.OnComponentBeginOverlap`
  (params (OverlappedComponent :type "PrimitiveComponent Object Reference") (OtherActor :type "Actor Object Reference") (OtherComp :type "PrimitiveComponent Object Reference") (OtherBodyIndex :type Integer) (bFromSweep :type Boolean) (SweepResult :type "HitResult Structure (by ref)"))
  (bind _returnvalue (`self.K2_GetActorLocation`))
  (bind _geometrycollectioncomponent (`self.GeometryCollectionComponent`))
  (`PrimitiveComponent.SetSimulatePhysics` _geometrycollectioncomponent true)
  (`PrimitiveComponent.AddImpulse` _geometrycollectioncomponent (0.0 0.0 100000.0) "None" false)
  (`NiagaraFunctionLibrary.SpawnSystemAtLocation` "/Game/FX/P_Fart.P_Fart" _returnvalue)
  (`GameplayStatics.PlaySoundAtLocation` "/Game/StarterContent/Audio/Explosion_Cue.Explosion_Cue" _returnvalue (struct) 1.0 1.0 0.0 null null null null)
  (`ActorComponent.K2_DestroyComponent` (`self.Box`))
  (`|SpawnActorFromClass` "BP_Car_GeometryCollection_GeometryCollection_Blueprint_C" (`KismetMathLibrary.MakeTransform` (0.0 0.0 0.0)) "Undefined" "OverrideRootScale" null null)
  (`KismetSystemLibrary.Delay` 5.0)
  (`self.K2_DestroyActor`))

(fn `UserConstructionScript`)